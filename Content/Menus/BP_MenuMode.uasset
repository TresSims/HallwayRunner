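; BP_MenuMode manages switching between the main menu and credits screens.
; On BeginPlay it creates and stores both widgets, showing only the main menu.
; SwitchToCredits and SwitchToMainMenu each clear all widgets, then add the stored target widget back to the viewport, reusing the same instances.
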(event EventBeginPlay
  (bind _returnvalue (UserInterface|CreateWidget "/Game/Menus/BP_MainMenu.BP_MainMenu_C"))
  (bind _output_get (Variables|Default|SetMM _returnvalue))
  (UserInterface|Viewport|AddtoViewport _output_get 0)
  (bind _returnvalue_2 (UserInterface|CreateWidget "/Game/Menus/BP_Credits.BP_Credits_C"))
  (Variables|Default|SetCredits _returnvalue_2))

(event EventTick
  (params (DeltaSeconds :type Float%20%28single-precision%29)))

(fn ConstructionScript)

(fn SwitchtoCredits
  (Viewport|RemoveAllWidgets)
  (UserInterface|Viewport|AddtoViewport (Variables|Default|GetCredits) 0))

(fn SwitchtoMainMenu
  (Viewport|RemoveAllWidgets)
  (UserInterface|Viewport|AddtoViewport (Variables|Default|GetMM) 0))