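; BP_BBully is a HallwayRunner enemy that steers toward the player.
; Every Tick it computes the normalized direction from its root to the Player's mesh and feeds it to FloatingPawnMovement as input, with no pathfinding.
; It also draws that direction as debug text at its own location each frame.
; The Player reference is not assigned anywhere in these graphs.
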(event EventBeginPlay)

(event Collision|EventActorBeginOverlap
  (params (OtherActor :type Actor%20Object%20Reference)))

(event EventTick
  (params (DeltaSeconds :type Float%20%28single-precision%29))
  (bind _defaultsceneroot (Variables|Default|GetDefaultSceneRoot))
  (bind _player (Variables|Default|Getplayer))
  (bind _returnvalue (Transformation|GetWorldLocation _defaultsceneroot))
  (bind _mesh (Variables|/Script/Engine.Character|GetMesh _player))
  (bind _returnvalue_2 (Transformation|GetWorldLocation _mesh))
  (bind _returnvalue_3 (- _returnvalue_2 _returnvalue))
  (bind _returnvalue_4 (Math|Vector|Normalize _returnvalue_3))
  (Rendering|Debug|DrawDebugString _returnvalue (Utilities|String|ToString(Vector) _returnvalue_4) 0 "(R=1.000000,G=0.802672,B=0.000000,A=1.000000)")
  (Class|PawnMovementComponent|AddInputVector (Variables|Default|GetFloatingPawnMovement) _returnvalue_4 false))

(fn ConstructionScript)