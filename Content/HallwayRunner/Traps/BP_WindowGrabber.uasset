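; BP_WindowGrabber is a hallway runner trap whose window swings open when the player approaches and which hurts them on contact.
; Overlap of the Detect volume by ThirdPersonCharacter sets a flag that is never cleared.
; While it is set, Tick repeatedly plays the OpenWindow timeline, whose curve drives the window mesh's roll.
; A separate Damage volume calls HandHit on the overlapping character, independently of the window's state.
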(event OnComponentBeginOverlap(Detect)
  (params (OverlappedComponent :type Primitive%20Component%20Object%20Reference) (OtherActor :type Actor%20Object%20Reference) (OtherComp :type Primitive%20Component%20Object%20Reference) (OtherBodyIndex :type Integer) (bFromSweep :type Boolean) (SweepResult :type Hit%20Result%20Structure%20%28by%20ref%29))
  (Utilities|Casting|CastToThirdPersonCharacter OtherActor)
  (Variables|Default|Setdetected true))

(event OnComponentBeginOverlap(Damage)
  (params (OverlappedComponent :type Primitive%20Component%20Object%20Reference) (OtherActor :type Actor%20Object%20Reference) (OtherComp :type Primitive%20Component%20Object%20Reference) (OtherBodyIndex :type Integer) (bFromSweep :type Boolean) (SweepResult :type Hit%20Result%20Structure%20%28by%20ref%29))
  (bind _asthird_person_character (Utilities|Casting|CastToThirdPersonCharacter OtherActor))
  (Default|HandHit _asthird_person_character))

(event EventBeginPlay)

(event Collision|EventActorBeginOverlap
  (params (OtherActor :type Actor%20Object%20Reference)))

(event EventTick
  (params (DeltaSeconds :type Float%20%28single-precision%29))
  (if (Variables|Default|Getdetected)
    (bind _windowopen (Timeline|OpenWindow Play)
      (:Update
        (Transformation|SetRelativeRotation (Variables|Default|GetWindowBase_SM_Window) (Math|Rotator|MakeRotator (* _windowopen 1e+02) 0.0 0.0) false false)))))

(fn ConstructionScript)