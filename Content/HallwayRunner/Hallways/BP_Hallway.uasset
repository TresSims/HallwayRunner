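; BP_Hallway is a hallway segment that chains random pieces together at runtime in the hallway runner.
; When ThirdPersonCharacter overlaps its Box, it rotates the door and spawns a random class from the Runner game mode's Doors array at SpawnPoint, with Passed ensuring this happens once.
; When BP_BBully overlaps the same Box, the segment destroys itself.
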(event OnComponentBeginOverlap(Box)
  (params (OverlappedComponent :type Primitive%20Component%20Object%20Reference) (OtherActor :type Actor%20Object%20Reference) (OtherComp :type Primitive%20Component%20Object%20Reference) (OtherBodyIndex :type Integer) (bFromSweep :type Boolean) (SweepResult :type Hit%20Result%20Structure%20%28by%20ref%29))
  (Utilities|FlowControl|Sequence
    (:then_0
      (Utilities|Casting|CastToThirdPersonCharacter OtherActor)
      (CallFunction|OpenDoor))
    (:then_1
      (Utilities|Casting|CastToBP_BBully OtherActor)
      (CallFunction|DestroyRoom))))

(event EventBeginPlay)

(event Collision|EventActorBeginOverlap
  (params (OtherActor :type Actor%20Object%20Reference)))

(event EventTick
  (params (DeltaSeconds :type Float%20%28single-precision%29)))

(fn ConstructionScript)

(fn OpenDoor
  (if (not (Variables|Default|GetPassed))
    (Transformation|AddLocalRotation (Variables|Default|GetSM_HallwayBase_Door) "0.000000,-90.000000, 0" false false)
    (Variables|Default|SetPassed true)
    (bind _asrunner (Utilities|Casting|CastToRunner (Game|GetGameMode)))
    (Game|SpawnActorfromClass (Utilities|Array|Get(acopy) (Variables|/Game/HallwayRunner/Runner.Runner_C|GetDoors _asrunner) (Math|Random|RandomInteger (Utilities|Array|Length (Variables|/Game/HallwayRunner/Runner.Runner_C|GetDoors _asrunner)))) (Transformation|GetWorldTransform (Variables|Default|GetSpawnPoint)) "Undefined" 0 0)))

(fn DestroyRoom
  (Actor|DestroyActor))